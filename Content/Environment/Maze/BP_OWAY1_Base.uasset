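; BP_OWAY1_Base is a maze element that flips a pair of maze platforms when it is enabled and unflips them when disabled.
; Both transitions are staggered, with the second platform following the first after a short delay.
; The construction script passes a Platform setting to each child platform.
; On the maze level's OnInitLevel event, it copies its Symbol to both platforms and applies it.
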(event Custom|onEnable_Event_0
  ;[1 1 1] Init
  (CallFunction|FlipPlatforms))

(event Custom|onDisable_Event_0
  ;[1 1 1] Init
  (CallFunction|UnflipPlatforms))

(event Custom|UnflipPlatforms
  ;[1 1 1] FlipPlatfomrs
  (Default|Unflip (Variables|Default|GetBP_MazePlatform))
  (Utilities|FlowControl|Delay 0.2)
  (Default|Unflip (Variables|Default|GetBP_MazePlatform1)))

(event Custom|OnInitLevel_Event_0
  ;[1 1 1] Init
  (CallFunction|ApplySymbol))

(event Custom|ApplySymbol
  (bind _bp_mazeplatform (Variables|Default|GetBP_MazePlatform))
  (bind _bp_mazeplatform1 (Variables|Default|GetBP_MazePlatform1))
  ;[1 1 1] ApplySymbol
  (Variables|/Game/Environment/Maze/BP_MazePlatform.BP_MazePlatform_C|Setsymbol _bp_mazeplatform (Variables|Default|Getsymbol))
  (Default|ApplySymbol _bp_mazeplatform)
  (Variables|/Game/Environment/Maze/BP_MazePlatform.BP_MazePlatform_C|Setsymbol _bp_mazeplatform1 (Variables|Default|Getsymbol))
  (Default|ApplySymbol _bp_mazeplatform1))

(event Custom|FlipPlatforms
  ;[1 1 1] FlipPlatfomrs
  (Default|Flip (Variables|Default|GetBP_MazePlatform))
  (Utilities|FlowControl|Delay 0.2)
  (Default|Flip (Variables|Default|GetBP_MazePlatform1)))

(event EventBeginPlay
  ;[1 1 1] Init
  (EventDispatchers|AssignOnEnable (delegate Custom|onEnable_Event_0))
  (EventDispatchers|AssignOnDisable (delegate Custom|onDisable_Event_0))
  (bind _returnvalue (Class|BPLevel|GetMazeLevel))
  (bind _asbp_level (Utilities|Casting|CastToBP_Level _returnvalue))
  (EventDispatchers|AssignOnInitLevel _asbp_level (delegate Custom|OnInitLevel_Event_0)))

(event Collision|EventActorBeginOverlap
  (params (OtherActor :type Actor%20Object%20Reference)))

(event EventTick
  (params (DeltaSeconds :type Float%20%28single-precision%29)))

(fn ConstructionScript
  (Variables|/Game/Environment/Maze/BP_MazePlatform.BP_MazePlatform_C|Setplatform (Variables|Default|GetBP_MazePlatform) (Variables|Default|Getplatform))
  (Variables|/Game/Environment/Maze/BP_MazePlatform.BP_MazePlatform_C|Setplatform (Variables|Default|GetBP_MazePlatform1) (Variables|Default|Getplatform1)))