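; BP_MazePlatform is a maze platform that can flip over and display a symbol color.
; Flip and Unflip rotate the Platform component in place in two eased MoveComponentTo steps through 90 degrees, separated by a short delay, with IsFlipped preventing repeats.
; ApplySymbol creates a dynamic instance of a debug obstacle material on the platform and sets its Color parameter from the Symbol's color.
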(event Custom|Flip
  (bind _platform (Variables|Default|Getplatform))
  (bind _relativelocation (Variables|/Script/Engine.SceneComponent|GetRelativeLocation _platform))
  (if (not (Variables|Default|GetisFlipped))
    (Components|MoveComponentTo _platform _relativelocation "0, 0,90.000000" false true 0.3 false)
    (Utilities|FlowControl|Delay 0.2)
    (Components|MoveComponentTo (Variables|Default|Getplatform) _relativelocation "0, 0,180.000000" false true 0.3 false)
    (Variables|Default|SetisFlipped true)))

(event Custom|Unflip
  (bind _platform (Variables|Default|Getplatform))
  (bind _relativelocation (Variables|/Script/Engine.SceneComponent|GetRelativeLocation _platform))
  (if (Variables|Default|GetisFlipped)
    (Components|MoveComponentTo _platform _relativelocation "0, 0,90.000000" false true 0.3 false)
    (Utilities|FlowControl|Delay 0.2)
    (Components|MoveComponentTo (Variables|Default|Getplatform) _relativelocation "0, 0, 0" false true 0.3 false)
    (Variables|Default|SetisFlipped false)))

(event Custom|ApplySymbol
  (bind _returnvalue (Rendering|Material|CreateDynamicMaterialInstance (Variables|Default|Getplatform) 0 "/Game/Environment/Maze/Materials/M_ObsticleDebug.M_ObsticleDebug" "None" :!class /Script/Engine.PrimitiveComponent))
  (Rendering|Material|SetVectorParameterValue _returnvalue "Color" (Math|Conversions|ToLinearColor(Color) (.color (Variables|Default|Getsymbol))) :!class /Script/Engine.MaterialInstanceDynamic))

(event EventTick
  (params (DeltaSeconds :type Float%20%28single-precision%29)))