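; Game mode for the maze level, managing player start, death resets and game over in a time-shift replay mechanic.
; BeginPlay generates BP_Maze and moves the player to BP_Start, then creates the first flux time shifter.
; Player death hands a previous shifter's recorded commands to a new AIRaiderController, shifts every time shifter and fires the scene reset.
; GameOver resets the level, possesses a fresh raider at the start and re-initializes the shifters.
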(event Custom|ShiftTimeOnReset
  ;[1 1 1] Shift time
  (for _array_element (Variables|Default|GettimeShifters)
    (Default|ShiftTime _array_element)))

(event Custom|SetFirstShifter
  ;[1 1 1] SetFirstTimeShifter
  (if (Utilities|Array|IsEmpty (Variables|Default|GettimeShifters))
    (bind _asbp_raider (Utilities|Casting|CastToBP_Raider (Game|Player|GetPlayerPawn 0)))
    (bind _timeshifter (CallFunction|CreateTimeShifter (Transformation|GetWorldTransform (Variables|/Script/Engine.Actor|GetRootComponent _asbp_raider))))
    (Default|ShiftTime _timeshifter)))

(event Custom|InitPlayerTransform
  (params (transform :type Transform))
  ;[1 1 1] Begin level
  (bind _output_get (Variables|Default|SetstartTransform transform))
  (bind _ascharacter (Utilities|Casting|CastToCharacter (Game|Player|GetPlayerPawn 0)))
  (Transformation|SetWorldTransform (Variables|/Script/Engine.Actor|GetRootComponent _ascharacter) _output_get false true)
  (CallFunction|Init))

(event Custom|OnPlayerDeathController
  ;[1 1 1] Init
  (if true
    _
    (else
      _))
  (CallFunction|SetupControllers)
  (CallFunction|ShiftTimeonReset)
  (Default|CallOnResetScene))

(event Custom|SetupControllers
  ;[1 1 1] setControllers
  (bind _result (Math|Integer|DecrementInt (Utilities|Array|LastIndex (Variables|Default|GettimeShifters)))
    (:%20%20
      (if (>= _result 0)
        (bind _asraider_controller (Utilities|Casting|CastToRaiderController (Variables|/Game/Environment/BP_FluxTimeShifter.BP_FluxTimeShifter_C|Getcontroller (Utilities|Array|Get(acopy) (Variables|Default|GettimeShifters) _result))))
        (bind _returnvalue (Game|SpawnActorfromClass "/Game/Raider/Blueprints/AIRaiderController.AIRaiderController_C" (Math|Transform|MakeTransform "0, 0, 0") "Undefined" 0 0))
        (Variables|/Game/Raider/Blueprints/AIRaiderController.AIRaiderController_C|Setcommands _returnvalue (Variables|/Game/Raider/Blueprints/RaiderController.RaiderController_C|Getcommands _asraider_controller))
        (Variables|/Game/Environment/BP_FluxTimeShifter.BP_FluxTimeShifter_C|Setcontroller (Utilities|Array|Get(acopy) (Variables|Default|GettimeShifters) _result) _returnvalue)))))

(event Custom|GameOver
  ;[1 1 1] GameOver
  (Class|GameModeBase|ResetLevel)
  (bind _raider (CallFunction|CreateRaider (Variables|Default|GetstartTransform)))
  (Pawn|Possess (Game|GetPlayerController 0) _raider)
  (CallFunction|Init))

(event Custom|Init
  ;[1 1 1] Init
  (Utilities|Array|Clear (Variables|Default|GettimeShifters))
  (CallFunction|SetFirstShifter)
  (bind _asraider_controller (Utilities|Casting|CastToRaiderController (Game|GetPlayerController 0)))
  (EventDispatchers|BindEventtoOnPlayerDeath _asraider_controller (delegate Custom|OnPlayerDeathController)))

(event EventBeginPlay
  ;[1 1 1] Begin level
  (bind _returnvalue (Actor|GetActorOfClass "/Script/RaiderOfTimeProto.BP_Maze"))
  (Utilities|IsValid _returnvalue
    (:Is%20Valid
      (Class|BPMaze|GenerateMaze _returnvalue)
      (bind _returnvalue_2 (Actor|GetActorOfClass "/Game/Environment/Maze/BP_Start.BP_Start_C"))
      (CallFunction|InitPlayerTransform (Transformation|GetWorldTransform (Variables|/Game/Environment/Maze/BP_Start.BP_Start_C|GetDefaultSceneRoot _returnvalue_2))))
    (:Is%20Not%20Valid
      (bind _ascharacter (Utilities|Casting|CastToCharacter (Game|Player|GetPlayerPawn 0)))
      (CallFunction|InitPlayerTransform (Transformation|GetWorldTransform (Variables|/Script/Engine.Character|GetCapsuleComponent _ascharacter))))))

(fn ConstructionScript)

(fn CreateTimeShifter
  (params (transform :type Transform))
  (bind _returnvalue (Game|SpawnActorfromClass "/Game/Environment/BP_FluxTimeShifter.BP_FluxTimeShifter_C" transform "Undefined" 0 0))
  (Utilities|Array|Add (Variables|Default|GettimeShifters) _returnvalue)
  (return _returnvalue))

(fn CreateRaider
  (params (transform :type Transform))
  (bind _returnvalue (Game|SpawnActorfromClass "/Game/Raider/Blueprints/BP_Raider.BP_Raider_C" transform "Undefined" 0 0))
  (return _returnvalue))