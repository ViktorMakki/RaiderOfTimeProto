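; BP_KSwitch is a maze switch on a platform base that activates and deactivates a linked symbol.
; On BeginPlay it binds its own enable and disable events to the child BP_Switch, and that switch's activate and deactivate events to SymbolToActivate.
; The construction script registers the switch component with the child BP_Platform_Base through AddChild.
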(event Custom|CustomEvent_3
  ;[1 1 1] Setup events
  (Class|Activable|Disable (stale EventBeginPlay _asbp_switch)))

(event Custom|CustomEvent_4
  ;[1 1 1] Setup events
  (Class|Activable|Enable (stale EventBeginPlay _asbp_switch)))

(event Custom|CustomEvent_5
  ;[1 1 1] Setup events
  (Class|Activable|Activate (Variables|Default|GetsymbolToActivate)))

(event Custom|CustomEvent_6
  ;[1 1 1] Setup events
  (Class|Activable|Deactivate (Variables|Default|GetsymbolToActivate)))

(event EventBeginPlay
  ;[1 1 1] Setup events
  (|CallParentFunction)
  (bind _asbp_switch (Utilities|Casting|CastToBP_Switch (Variables|/Script/Engine.ChildActorComponent|GetChildActor (Variables|Default|GetBP_Switch))))
  (EventDispatchers|BindEventtoOnDisable (delegate Custom|CustomEvent_3))
  (EventDispatchers|BindEventtoOnEnable (delegate Custom|CustomEvent_4))
  (EventDispatchers|BindEventtoOnActivate _asbp_switch (delegate Custom|CustomEvent_5))
  (EventDispatchers|BindEventtoOnDeactivate _asbp_switch (delegate Custom|CustomEvent_6)))

(event Collision|EventActorBeginOverlap
  (params (OtherActor :type Actor%20Object%20Reference))
  (|CallParentFunction OtherActor) ; This node is disabled and will not be called.\nDrag off pins to build functionality.
)

(event EventTick
  (params (DeltaSeconds :type Float%20%28single-precision%29))
  (|CallParentFunction DeltaSeconds) ; This node is disabled and will not be called.\nDrag off pins to build functionality.
)

(fn ConstructionScript
  (|CallParentFunction)
  (bind _asbp_platform_base (Utilities|Casting|CastToBP_Platform_Base (Variables|/Script/Engine.ChildActorComponent|GetChildActor (Variables|Default|GetBP_Platform_Base))))
  (Default|AddChild _asbp_platform_base (Variables|Default|GetBP_Switch)))