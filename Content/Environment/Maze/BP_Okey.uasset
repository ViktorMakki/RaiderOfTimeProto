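; BP_Okey is a maze object that shows its own symbol color and that of the symbol it is set to activate.
; On BeginPlay it binds to the symbol-changed event, which calls ApplySymbol.
; ApplySymbol creates dynamic M_ObsticleDebug material instances, tinting StaticMesh with its Symbol color and, when SymbolToActivate is valid, StaticMesh1 with that target's color.
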(event Custom|ApplySymbol
  (bind _returnvalue (Rendering|Material|CreateDynamicMaterialInstance (Variables|Default|GetStaticMesh) 0 "/Game/Environment/Maze/Materials/M_ObsticleDebug.M_ObsticleDebug" "None" :!class /Script/Engine.PrimitiveComponent))
  (Rendering|Material|SetVectorParameterValue _returnvalue "Color" (Math|Conversions|ToLinearColor(Color) (.color (Utilities|Struct|BreakSymbol (Variables|Default|Getsymbol)))) :!class /Script/Engine.MaterialInstanceDynamic)
  (bind _symboltoactivate (Variables|Default|GetsymbolToActivate)
    (:then
      (bind _returnvalue_2 (Rendering|Material|CreateDynamicMaterialInstance (Variables|Default|GetStaticMesh1) 0 "/Game/Environment/Maze/Materials/M_ObsticleDebug.M_ObsticleDebug" "None" :!class /Script/Engine.PrimitiveComponent))
      (Rendering|Material|SetVectorParameterValue _returnvalue_2 "Color" (Math|Conversions|ToLinearColor(Color) (.color (Class|SymbolRule|GetSymbol _symboltoactivate))) :!class /Script/Engine.MaterialInstanceDynamic))
    (:else)))

(event Custom|CustomEvent_0
  (CallFunction|ApplySymbol))

(event EventBeginPlay
  (EventDispatchers|BindEventtoSymbolChanged (delegate Custom|CustomEvent_0)))

(event Collision|EventActorBeginOverlap
  (params (OtherActor :type Actor%20Object%20Reference)))

(event EventTick
  (params (DeltaSeconds :type Float%20%28single-precision%29)))

(fn ConstructionScript)