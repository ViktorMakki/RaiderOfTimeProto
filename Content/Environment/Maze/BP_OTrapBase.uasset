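; Base maze trap actor with platforms that take on the color of the trap's Symbol and can flip over.
; On BeginPlay it binds to symbol changes, and ApplySymbol then gives each platform a dynamic debug material tinted to that color.
; Flip and Unflip, guarded by IsFlipped, rotate platforms through 90 degrees to 180 or back, using latent MoveComponentTo and Delay nodes inside the platform loop.
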(event Custom|ApplySymbol
  (bind _platforms (Variables|Default|Getplatforms))
  ;[1 1 1] ApplySymbol
  (if (not (Utilities|Array|IsEmpty _platforms))
    (for _array_element _platforms
      (bind _returnvalue (Rendering|Material|CreateDynamicMaterialInstance _array_element 0 "/Game/Environment/Maze/Materials/M_ObsticleDebug.M_ObsticleDebug" "None" :!class /Script/Engine.PrimitiveComponent))
      (Rendering|Material|SetVectorParameterValue _returnvalue "Color" (Math|Conversions|ToLinearColor(Color) (.color (Variables|Default|Getsymbol))) :!class /Script/Engine.MaterialInstanceDynamic))))

(event Custom|CustomEvent_0
  ;[1 1 1] BeginPlay
  (CallFunction|ApplySymbol))

(event Custom|Flip
  ;[1 1 1] Flip
  (if (not (or (Variables|Default|GetisFlipped) (Utilities|Array|IsEmpty (Variables|Default|Getplatforms))))
    (for _array_element (Variables|Default|Getplatforms)
      (Components|MoveComponentTo _array_element (Variables|/Script/Engine.SceneComponent|GetRelativeLocation _array_element) "0, 0,90.000000" false true 0.3 false)
      (Utilities|FlowControl|Delay 0.2)
      (Components|MoveComponentTo _array_element (Variables|/Script/Engine.SceneComponent|GetRelativeLocation _array_element) "0, 0,180.000000" false true 0.3 false)
      (Utilities|FlowControl|Delay 0.2)
      (Variables|Default|SetisFlipped true))))

(event Custom|Unflip
  ;[1 1 1] Unflip
  (if (and (Variables|Default|GetisFlipped) (not (Utilities|Array|IsEmpty (Variables|Default|Getplatforms))))
    (for _array_element (Variables|Default|Getplatforms)
      (Components|MoveComponentTo _array_element (Variables|/Script/Engine.SceneComponent|GetRelativeLocation _array_element) "0, 0,90.000000" false true 0.3 false)
      (Utilities|FlowControl|Delay 0.2)
      (Components|MoveComponentTo _array_element (Variables|/Script/Engine.SceneComponent|GetRelativeLocation _array_element) "0, 0, 0" false true 0.3 false)
      (Utilities|FlowControl|Delay 0.2)
      (Variables|Default|SetisFlipped false))))

(event EventBeginPlay
  ;[1 1 1] BeginPlay
  (EventDispatchers|BindEventtoSymbolChanged (delegate Custom|CustomEvent_0)))

(event Collision|EventActorBeginOverlap
  (params (OtherActor :type Actor%20Object%20Reference)))

(event EventTick
  (params (DeltaSeconds :type Float%20%28single-precision%29)))

(fn ConstructionScript)