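; BP_FluxTimeShifter is an environment actor that "reincarnates" a Raider pawn at its own location.
; At BeginPlay it caches the first player controller and that player's BP_Raider.
; ShiftTime asks GM_Maze to create a Raider at the actor's transform, has the cached controller possess it, then destroys the previous Raider.
; OnReset destroys the shifter, along with the controller if it is an AIController.
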(event Custom|ShiftTime
  ;[1 1 1] ShiftTimeReincarnate
  (bind _asgm_maze (Utilities|Casting|CastToGM_Maze (Game|GetGameMode)))
  (bind _raider (Default|CreateRaider _asgm_maze (Transformation|GetWorldTransform (Variables|Default|GetDefaultSceneRoot))))
  (bind _controller (Variables|Default|Getcontroller)
    (:then
      (Pawn|Possess _controller _raider)
      (bind _raider_2 (Variables|Default|Getraider)
        (:then
          (Actor|DestroyActor _raider_2))
        (:else
          _))
      (Variables|Default|Setraider _raider))
    (:else)))

(event EventBeginPlay
  ;[1 1 1] Construction
  (Variables|Default|Setcontroller (Game|GetPlayerController 0))
  (bind _asbp_raider (Utilities|Casting|CastToBP_Raider (Game|Player|GetPlayerPawn 0)))
  (Variables|Default|Setraider _asbp_raider))

(event Collision|EventActorBeginOverlap
  (params (OtherActor :type Actor%20Object%20Reference)))

(event EventTick
  (params (DeltaSeconds :type Float%20%28single-precision%29)))

(event EventOnReset
  ;[1 1 1] Reset
  (bind _asaicontroller (Utilities|Casting|CastToAIController (Variables|Default|Getcontroller))
    (:then
      (Actor|DestroyActor _asaicontroller))
    (:CastFailed
      _))
  (Actor|DestroyActor))

(fn ConstructionScript)