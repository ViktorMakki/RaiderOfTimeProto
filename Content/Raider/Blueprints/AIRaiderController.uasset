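; AI controller that drives a BP_Raider by playing back a timed list of commands.
; Each tick accumulates time against the current command's delta, then advances and applies the next command's movement direction and jump, slide or interact action.
; Movement input is applied every tick until the list runs out, after which it calls Die on the raider.
; GM_Maze's scene reset event rewinds playback to the start.
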(event Custom|ExecuteCommand
  (params (deltaTime :type Float%20%28single-precision%29))
  (bind _index (Variables|Default|Getindex))
  (bind _commands (Variables|Default|Getcommands))
  ;[1 1 1] Execute Command
  (bind _output_get (Variables|Default|Setdelta (+ (Variables|Default|Getdelta) deltaTime)))
  (if (<= (.delta (Utilities|Array|Get(acopy) (Variables|Default|Getcommands) (Variables|Default|Getindex))) _output_get)
    (Variables|Default|Setdelta 0.0)
    (Math|Integer|IncrementInt _index
      (:%20%20
        (if (< _index (Utilities|Array|Length _commands))
          (CallFunction|ExecNewCommand (Utilities|Array|Get(acopy) _commands (Variables|Default|Getindex)))
          (else
            (Variables|Default|SetisDone true)))))))

(event Custom|ExecNewCommand
  (params (command :type S%20Control%20Command%20Structure))
  ;[1 1 1] Execute Command
  (Variables|Default|SetmoveDirection (Math|Vector|MakeVector (.x (.direction command)) (.y (.direction command)) 0.0))
  (bind _asbp_raider (Utilities|Casting|CastToBP_Raider (Pawn|GetControlledPawn)))
  (switch Utilities|FlowControl|Switch|SwitchonE_Commands (.command command)
    (:NewEnumerator0
      (Default|JumpEvent _asbp_raider))
    (:NewEnumerator1
      (Default|Slide _asbp_raider))
    (:NewEnumerator3
      (Default|Interact _asbp_raider))))

(event Custom|onResetScenario
  ;[1 1 1] Construct
  (Variables|Default|Setindex 0)
  (Variables|Default|Setdelta 0.0)
  (Variables|Default|SetmoveDirection "0, 0, 0")
  (Variables|Default|SetisDone false))

(event EventBeginPlay
  ;[1 1 1] Construct
  (bind _asgm_maze (Utilities|Casting|CastToGM_Maze (Game|GetGameMode)))
  (EventDispatchers|BindEventtoOnResetScene _asgm_maze (delegate Custom|onResetScenario)))

(event EventTick
  (params (DeltaSeconds :type Float%20%28single-precision%29))
  (bind _returnvalue (Pawn|GetControlledPawn))
  ;[1 1 1] Update
  (if (Variables|Default|GetisDone)
    (bind _asbp_raider (Utilities|Casting|CastToBP_Raider (Pawn|GetControlledPawn)))
    (Default|Die _asbp_raider)
    (else
      (CallFunction|ExecuteCommand DeltaSeconds)
      (Utilities|IsValid _returnvalue
        (:Is%20Valid
          (Pawn|Input|AddMovementInput _returnvalue (Variables|Default|GetmoveDirection) 1.0 false))))))

(fn ConstructionScript)