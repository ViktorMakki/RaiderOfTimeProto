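; BP_Maze is an actor that builds a tile-based maze in the level when play begins.
; It calls GenerateMaze with a fixed-size grid, then loops over the returned columns and tiles, spawning PathClass or WallClass actors at index times TileSize.
; Each spawned tile attaches to the maze actor with KeepRelative rules, so its grid position becomes an offset from that actor.
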(event EventBeginPlay
  (bind _tilesize (Variables|Default|GettileSize))
  ;[1 1 1] Generate Maze
  (bind _returnvalue (Class|MazeGenerator|GenerateMaze (Utilities|Struct|MakeMazeGeneratorData 21 21)))
  (for (_array_element _array_index) _returnvalue
    (for (_array_element_2 _array_index_2) (.tiles _array_element)
      (switch Utilities|FlowControl|Switch|SwitchonMazeTileType _array_element_2
        (:PATH
          (bind _returnvalue_2 (Game|SpawnActorfromClass (Variables|Default|GetpathClass) (Math|Transform|MakeTransform (Math|Vector|MakeVector (* _array_index _tilesize) (* _tilesize _array_index_2) 0.0)) "Undefined" 0 0))
          (Transformation|AttachActorToActor _returnvalue_2 self "None" "KeepRelative" "KeepRelative" "KeepRelative" false))
        (:WALL
          (bind _returnvalue_3 (Game|SpawnActorfromClass (Variables|Default|GetwallClass) (Math|Transform|MakeTransform (Math|Vector|MakeVector (* _array_index _tilesize) (* _tilesize _array_index_2) 0.0)) "Undefined" 0 0))
          (Transformation|AttachActorToActor _returnvalue_3 self "None" "KeepRelative" "KeepRelative" "KeepRelative" false))))))

(event Collision|EventActorBeginOverlap
  (params (OtherActor :type Actor%20Object%20Reference)))

(event EventTick
  (params (DeltaSeconds :type Float%20%28single-precision%29)))

(fn ConstructionScript)