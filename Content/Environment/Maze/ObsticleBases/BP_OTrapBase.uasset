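; BP_OTrapBase is a base maze obstacle trap that controls a set of symbol-bearing, flippable platforms.
; On BeginPlay it binds to its symbol-changed, enable and disable events.
; A symbol change copies the current symbol to every platform at once.
; Enabling unflips the platforms and disabling flips them, using a ForEachDelay loop to stagger them one after another.
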(event Custom|ApplySymbol
  ;[1 1 1] ApplySymbol
  (for _array_element (Variables|Default|Getplatforms)
    (Default|SetSymbol _array_element (Class|Obstilce|GetSymbol))))

(event Custom|CustomEvent_0
  ;[1 1 1] BeginPlay
  (CallFunction|ApplySymbol))

(event Custom|CustomEvent_1
  ;[1 1 1] BeginPlay
  (CallFunction|Unflip))

(event Custom|Flip
  ;[1 1 1] Flip
  (bind _arrayelement (Utilities|ForEachDelay (Variables|Default|Getplatforms) 0.2)
    (:LoopBody
      (Default|Flip _arrayelement))))

(event Custom|CustomEvent_2
  ;[1 1 1] BeginPlay
  (CallFunction|Flip))

(event Custom|Unflip
  ;[1 1 1] Unflip
  (bind _arrayelement (Utilities|ForEachDelay (Variables|Default|Getplatforms) 0.2)
    (:LoopBody
      (Default|Unflip _arrayelement))))

(event EventBeginPlay
  ;[1 1 1] BeginPlay
  (EventDispatchers|BindEventtoSymbolChanged (delegate Custom|CustomEvent_0))
  (EventDispatchers|BindEventtoOnEnable (delegate Custom|CustomEvent_1))
  (EventDispatchers|BindEventtoOnDisable (delegate Custom|CustomEvent_2)))

(event Collision|EventActorBeginOverlap
  (params (OtherActor :type Actor%20Object%20Reference)))

(event EventTick
  (params (DeltaSeconds :type Float%20%28single-precision%29)))

(fn ConstructionScript)