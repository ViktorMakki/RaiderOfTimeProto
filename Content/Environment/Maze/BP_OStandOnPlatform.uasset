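; A maze pressure plate that activates when something overlaps its box and deactivates when the overlap ends.
; It binds its activate and deactivate dispatchers to push the static mesh down or back up with timed MoveComponentTo nodes.
; An IsMoving flag lets a trigger arriving mid-movement call Return on the opposite move, reversing it rather than starting a new one.
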(event OnComponentBeginOverlap(Box)
  (params (OverlappedComponent :type Primitive%20Component%20Object%20Reference) (OtherActor :type Actor%20Object%20Reference) (OtherComp :type Primitive%20Component%20Object%20Reference) (OtherBodyIndex :type Integer) (bFromSweep :type Boolean) (SweepResult :type Hit%20Result%20Structure%20%28by%20ref%29))
  ;[1 1 1] OnStandOn
  (Class|BPObsticle|Activate))

(event OnComponentEndOverlap(Box)
  (params (OverlappedComponent :type Primitive%20Component%20Object%20Reference) (OtherActor :type Actor%20Object%20Reference) (OtherComp :type Primitive%20Component%20Object%20Reference) (OtherBodyIndex :type Integer))
  ;[1 1 1] OnStandOn
  (Class|BPObsticle|Deactivate))

(event Custom|onActivate_Event
  ;[1 1 1] Init
  (CallFunction|PushDown))

(event Custom|PushUp
  ;[1 1 1] Movement
  (if (Variables|Default|GetisMoving)
    (Components|MoveComponentTo (Variables|Default|GetStaticMesh) "0,0.000000,-5.000000" "0, 0, 0" false false 0.6 false) ; enters at Return
    (else
      (Variables|Default|SetisMoving true)
      (Components|MoveComponentTo (Variables|Default|GetStaticMesh) "0,0.000000,20.000000" "0, 0, 0" false false 0.6 false)
      (Variables|Default|SetisMoving false))))

(event Custom|onDeactivate_Event
  ;[1 1 1] Init
  (CallFunction|PushUp))

(event Custom|PushDown
  ;[1 1 1] Movement
  (if (Variables|Default|GetisMoving)
    (Components|MoveComponentTo (Variables|Default|GetStaticMesh) "0,0.000000,20.000000" "0, 0, 0" false false 0.6 false) ; enters at Return
    (else
      (Variables|Default|SetisMoving true)
      (Components|MoveComponentTo (Variables|Default|GetStaticMesh) "0,0.000000,-5.000000" "0, 0, 0" false false 0.6 false)
      (Variables|Default|SetisMoving false))))

(event EventBeginPlay
  ;[1 1 1] Init
  (EventDispatchers|AssignOnActivate (delegate Custom|onActivate_Event))
  (EventDispatchers|AssignOnDeactivate (delegate Custom|onDeactivate_Event)))

(fn ConstructionScript)