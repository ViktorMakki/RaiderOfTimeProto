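; Base platform Blueprint for maze obstacles that can flip over and be color-coded by a symbol.
; Flip and Unflip play separate timelines that roll the Platform component between 0 and 180 degrees.
; AddChild attaches a child actor to the Platform, keeping relative location and rotation but world scale, while SetSymbol tints it through a dynamic instance of the debug obstacle material.
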(event Custom|Unflip
  ;[1 1 1] Unflip
  (bind _newtrack_0 (Timeline|Timeline_0 PlayFromStart)
    (:Update
      (Transformation|SetRelativeRotation (Variables|Default|Getplatform) (Math|Rotator|MakeRotator (* (- 1.0 _newtrack_0) 1.8e+02) 0.0 0.0) false false))))

(event Custom|Flip
  ;[1 1 1] Flip
  (bind _newtrack_0 (Timeline|FlipTimeLine PlayFromStart)
    (:Update
      (Transformation|SetRelativeRotation (Variables|Default|Getplatform) (Math|Rotator|MakeRotator (* _newtrack_0 1.8e+02) 0.0 0.0) false false))))

(fn ConstructionScript)

(fn AddChild
  (params (childActor :type Child%20Actor%20Component%20Object%20Reference))
  (Transformation|AttachComponentToComponent (Variables|/Script/Engine.ChildActorComponent|GetChildActor childActor) (Variables|Default|Getplatform) "None" "KeepRelative" "KeepRelative" "KeepWorld" false))

(fn SetSymbol
  (params (symbol :type Symbol%20Structure))
  (bind _returnvalue (Rendering|Material|CreateDynamicMaterialInstance (Variables|Default|Getplatform) 0 "/Game/Environment/Maze/Materials/M_ObsticleDebug.M_ObsticleDebug" "None" :!class /Script/Engine.PrimitiveComponent))
  (Rendering|Material|SetVectorParameterValue _returnvalue "Color" (Math|Conversions|ToLinearColor(Color) (.color symbol)) :!class /Script/Engine.MaterialInstanceDynamic))