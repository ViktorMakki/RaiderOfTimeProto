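; Maze trap with two sliding saws that kills BP_Raider characters when triggered.
; A Raider overlapping the actor calls Activate, and the bound OnActivate event runs the trap.
; Both saws snap inward, pause, then ease back out before calling Deactivate.
; A single box overlap query, fired as the saws start moving rather than following their motion, kills every Raider in the area.
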(event Custom|MoveSaw
  ;[1 1 1] Activate Trap
  (Components|MoveComponentTo (Variables|Default|GetSaw1) "0,-75.000000,150.000000" "0, 0, 0" false false 0.1 false)
  (Utilities|FlowControl|Delay 0.5)
  (Components|MoveComponentTo (Variables|Default|GetSaw1) "0,-300.000000,150.000000" "0, 0, 0" false true 1.0 false)
  (Class|BPObsticle|Deactivate))

(event Custom|MoveSaw2
  ;[1 1 1] Activate Trap
  (Components|MoveComponentTo (Variables|Default|GetSaw2) "0,75.000000,150.000000" "0, 0, 0" false false 0.1 false)
  (Utilities|FlowControl|Delay 0.5)
  (Components|MoveComponentTo (Variables|Default|GetSaw2) "0,300.000000,150.000000" "0, 0, 0" false true 1.0 false)
  (Class|BPObsticle|Deactivate))

(event Custom|onActivate_Event
  ;[1 1 1] Init
  (CallFunction|ActivateTrap))

(event Custom|ActivateTrap
  ;[1 1 1] Activate Trap
  (CallFunction|MoveSaw)
  (CallFunction|MoveSaw2)
  (bind _outactors (Collision|BoxOverlapActors (Transformation|GetWorldLocation (Variables|Default|GetBox)) "300.000000,300.000000,30.000000" (Utilities|Array|MakeArray "ObjectTypeQuery3") "/Game/Raider/Blueprints/BP_Raider.BP_Raider_C" :!class /Script/Engine.KismetSystemLibrary))
  (for _array_element _outactors
    (bind _asbp_raider (Utilities|Casting|CastToBP_Raider _array_element))
    (Default|Die _asbp_raider)))

(event EventBeginPlay
  ;[1 1 1] Init
  (EventDispatchers|AssignOnActivate (delegate Custom|onActivate_Event)))

(event Collision|EventActorBeginOverlap
  (params (OtherActor :type Actor%20Object%20Reference))
  ;[1 1 1] On Overlap
  (Utilities|Casting|CastToBP_Raider OtherActor)
  (Class|BPObsticle|Activate))

(fn ConstructionScript)