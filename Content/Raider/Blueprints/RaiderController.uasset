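; Player controller for the maze raider that forwards move, jump, slide and time-shifter input to BP_Raider while recording a command history.
; Tick accumulates time on the current command and, when command or direction changes, stamps the last entry with duration and pawn location, then appends a new one.
; History resets on possess, BeginPlay and GM_Maze's OnResetScene.
; Pawn death is relayed through the OnPlayerDeath dispatcher.
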(event Custom|ResetController
  ;[1 1 1] Reset
  (bind _output_get (Variables|Default|SetlastCommand (Utilities|Struct|MakeS_ControlCommand 0.0 "NewEnumerator2" "(X=0.000000,Y=0.000000)" "0.000000,0.000000,0.000000")))
  (Variables|Default|Setcommands (Utilities|Array|MakeArray (|Copy _output_get)))
  (bind _asbp_raider (Utilities|Casting|CastToBP_Raider (Pawn|GetControlledPawn)))
  (EventDispatchers|BindEventtoOnDeath _asbp_raider (delegate Custom|PlayerDeath)))

(event Custom|PlayerDeath
  ;[1 1 1] Reset
  (Default|CallOnPlayerDeath))

(event EventBeginPlay
  ;[1 1 1] Reset
  (CallFunction|ResetController)
  (bind _asgm_maze (Utilities|Casting|CastToGM_Maze (Game|GetGameMode)))
  (EventDispatchers|BindEventtoOnResetScene _asgm_maze (delegate Custom|ResetController)))

(event EventTick
  (params (DeltaSeconds :type Float%20%28single-precision%29))
  (bind _commands (Variables|Default|Getcommands))
  (bind _commands_2 (Variables|Default|Getcommands))
  (bind _returnvalue (Utilities|Array|LastIndex _commands))
  (bind _returnvalue_2 (Utilities|Array|LastIndex _commands_2))
  (bind _output (Utilities|Array|Get(acopy) _commands _returnvalue))
  (bind _output_2 (Utilities|Array|Get(acopy) _commands_2 _returnvalue_2))
  ;[1 1 1] Updtate
  (bind _output_get (Variables|Default|SetlastCommand (Utilities|Struct|MakeS_ControlCommand (+ (.delta (Variables|Default|GetlastCommand)) DeltaSeconds) (.command (Variables|Default|GetlastCommand)) (.direction (Variables|Default|GetlastCommand)) "0.000000,0.000000,0.000000")))
  (if (not (and (Utilities|Enum|Equal(Enum) (.command _output_get) (.command _output)) (Class|KismetMathLibrary|EqualExactlyVector2DVector2D (.direction _output_get) (.direction _output))))
    (bind _output_get_2 (Variables|Default|SetlastCommand (Utilities|Struct|MakeS_ControlCommand (.delta (Variables|Default|GetlastCommand)) (.command (Variables|Default|GetlastCommand)) (.direction (Variables|Default|GetlastCommand)) "0.000000,0.000000,0.000000")))
    (Utilities|Array|SetArrayElem _commands_2 _returnvalue_2 (Utilities|Struct|MakeS_ControlCommand (.delta (Variables|Default|GetlastCommand)) (.command _output_2) (.direction _output_2) (Transformation|GetActorLocation (Pawn|GetControlledPawn))))
    (Utilities|Array|Add (Variables|Default|Getcommands) (|Copy _output_get_2))
    (Variables|Default|SetlastCommand (Utilities|Struct|MakeS_ControlCommand 0.0 "NewEnumerator2" (.direction (Variables|Default|GetlastCommand)) "0.000000,0.000000,0.000000"))))

(event EventPossess
  (params (PossessedPawn :type Pawn%20Object%20Reference))
  ;[1 1 1] OnPosess
  (CallFunction|ResetController))

(event Input|ActionEvents|InputActionslide
  (params (Key :type Key%20Structure :default "None"))
  ;[1 1 1] SlideControl
  (:Pressed
    (Variables|Default|SetlastCommand (Utilities|Struct|MakeS_ControlCommand (.delta (Variables|Default|GetlastCommand)) "NewEnumerator1" (.direction (Variables|Default|GetlastCommand)) "0.000000,0.000000,0.000000"))
    (bind _asbp_raider (Utilities|Casting|CastToBP_Raider (Pawn|GetControlledPawn)))
    (Default|Slide _asbp_raider)))

(event Input|ActionEvents|InputActionTimeShifter
  (params (Key :type Key%20Structure :default "None"))
  ;[1 1 1] TimeShifterControl
  (:Pressed
    (bind _asbp_raider (Utilities|Casting|CastToBP_Raider (Pawn|GetControlledPawn)))
    (Default|PutTimeShifter _asbp_raider)))

(event Input|ActionEvents|InputActionJump
  (params (Key :type Key%20Structure :default "None"))
  ;[1 1 1] JumpControl
  (:Pressed
    (Variables|Default|SetlastCommand (Utilities|Struct|MakeS_ControlCommand (.delta (Variables|Default|GetlastCommand)) "NewEnumerator0" (.direction (Variables|Default|GetlastCommand)) "0.000000,0.000000,0.000000"))
    (bind _asbp_raider (Utilities|Casting|CastToBP_Raider (Pawn|GetControlledPawn)))
    (Default|JumpEvent _asbp_raider)))

(event Input|AxisEvents|InputAxisMoveForward
  (params (AxisValue :type Float%20%28single-precision%29))
  ;[1 1 1] MovementControl
  (bind _asbp_raider (Utilities|Casting|CastToBP_Raider (Pawn|GetControlledPawn)))
  (Default|MoveForeward _asbp_raider AxisValue)
  (Variables|Default|SetlastCommand (Utilities|Struct|MakeS_ControlCommand (.delta (Variables|Default|GetlastCommand)) (.command (Variables|Default|GetlastCommand)) (Math|Vector2D|MakeVector2D AxisValue (stale Input|AxisEvents|InputAxisMoveRight AxisValue)) "0.000000,0.000000,0.000000")))

(event Input|AxisEvents|InputAxisMoveRight
  (params (AxisValue :type Float%20%28single-precision%29))
  ;[1 1 1] MovementControl
  (bind _asbp_raider (Utilities|Casting|CastToBP_Raider (Pawn|GetControlledPawn)))
  (Default|MoveRight _asbp_raider AxisValue)
  (Variables|Default|SetlastCommand (Utilities|Struct|MakeS_ControlCommand (.delta (Variables|Default|GetlastCommand)) (.command (Variables|Default|GetlastCommand)) (Math|Vector2D|MakeVector2D (stale Input|AxisEvents|InputAxisMoveForward AxisValue) AxisValue) "0.000000,0.000000,0.000000")))

(fn ConstructionScript)