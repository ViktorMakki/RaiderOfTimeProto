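; BP_OGate is a maze gate with two door halves that slide apart when activated.
; On BeginPlay it subscribes to activation and symbol-change notifications.
; Activation moves each half in opposite directions over a short timed component move.
; ApplySymbol tints both halves with the symbol's color through dynamic instances of a debug obstacle material.
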(event Custom|ApplySymbol
  (bind _symbol (Variables|Default|Getsymbol))
  (bind _color (Utilities|Struct|BreakSymbol _symbol))
  (bind _returnvalue (Math|Conversions|ToLinearColor(Color) _color))
  (bind _returnvalue_2 (Rendering|Material|CreateDynamicMaterialInstance (Variables|Default|GethalfDoor1) 0 "/Game/Environment/Maze/Materials/M_ObsticleDebug.M_ObsticleDebug" "None" :!class /Script/Engine.PrimitiveComponent))
  (Rendering|Material|SetVectorParameterValue _returnvalue_2 "Color" _returnvalue :!class /Script/Engine.MaterialInstanceDynamic)
  (bind _returnvalue_3 (Rendering|Material|CreateDynamicMaterialInstance (Variables|Default|GethalfDoor2) 0 "/Game/Environment/Maze/Materials/M_ObsticleDebug.M_ObsticleDebug" "None" :!class /Script/Engine.PrimitiveComponent))
  (Rendering|Material|SetVectorParameterValue _returnvalue_3 "Color" _returnvalue :!class /Script/Engine.MaterialInstanceDynamic))

(event Custom|MoveDoor1
  (Components|MoveComponentTo (Variables|Default|GethalfDoor1) "0,215.000000,300.000000" "0, 0, 0" false false 0.5 false))

(event Custom|MoveDoor2
  (Components|MoveComponentTo (Variables|Default|GethalfDoor2) "0,-215.000000,300.000000" "0, 0, 0" false false 0.5 false))

(event Custom|onActivate_Event_0
  (CallFunction|MoveDoor1)
  (CallFunction|MoveDoor2))

(event EventBeginPlay
  (EventDispatchers|AssignOnActivate (delegate Custom|onActivate_Event_0))
  (EventDispatchers|BindEventtoSymbolChanged (EventDispatchers|CreateEvent :!event Custom|ApplySymbol)))

(event Collision|EventActorBeginOverlap
  (params (OtherActor :type Actor%20Object%20Reference)))

(event EventTick
  (params (DeltaSeconds :type Float%20%28single-precision%29)))

(fn ConstructionScript)