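; BP_Maze is a maze actor that generates a tile-based layout and spawns the actors that make it up.
; Generate stores the result of GenerateMaze, built from MazeConstructionData, in MazeData.
; SpawnActors places doors from their own list, rotating horizontal ones, then fills the non-door tiles on a TileSize grid.
; Each piece uses a random class from TileActorTypeMap for its tile type and is attached to the maze actor.
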(event Custom|Generate
  ;[1 1 1] Generate Maze
  (bind _returnvalue (Class|MazeGenerator|GenerateMaze (Variables|Default|GetmazeConstructionData)))
  (Variables|Default|SetmazeData _returnvalue))

(event Custom|SpawnActors
  (bind _tilesize (Variables|Default|GettileSize))
  ;[1 1 1] Spawn actors
  (CallFunction|CreateDoors)
  (for (_array_element _array_index) (.tiles (Variables|Default|GetmazeData))
    (for (_array_element_2 _array_index_2) (.tiles _array_element)
      (if (not (Utilities|Enum|Equal(Enum) (.tile _array_element_2) "DOOR"))
        (CallFunction|CreateChildActor (.tile _array_element_2) (Math|Transform|MakeTransform (Math|Vector|MakeVector (* _array_index _tilesize) (* _tilesize _array_index_2) 0.0)))))))

(event Custom|CreateChildActor
  (params (tileType :type MazeTileType%20Enum :default "WALL") (transform :type Transform))
  (bind _tileactortypemap (Variables|Default|GettileActorTypeMap))
  (bind (_value _returnvalue) (Utilities|Map|Find (.map _tileactortypemap) tileType))
  ;[1 1 1] Spawn actors
  (if _returnvalue
    (if (Utilities|Array|IsNotEmpty (.actortypes _value))
      (bind _returnvalue_2 (Game|SpawnActorfromClass (Utilities|Array|Get(acopy) (.actortypes _value) (Math|Random|RandomIntegerinRange 0 (- (Utilities|Array|Length (.actortypes _value)) 1))) transform "Undefined" 0 0))
      (Transformation|AttachActorToActor _returnvalue_2 self "None" "KeepRelative" "KeepRelative" "KeepRelative" true))))

(event Custom|CreateDoors
  (bind _tilesize (Variables|Default|GettileSize))
  ;[1 1 1] Spawn actors
  (for _array_element (.doors (Variables|Default|GetmazeData))
    (if (.ishorizontal _array_element)
      (CallFunction|CreateChildActor "DOOR" (Math|Transform|MakeTransform (Math|Vector|MakeVector (* (.x (.location _array_element)) _tilesize) (* (.y (.location _array_element)) _tilesize) 0.0) "0,90.000000, 0"))
      (else
        (CallFunction|CreateChildActor "DOOR" (Math|Transform|MakeTransform (Math|Vector|MakeVector (* (.x (.location _array_element)) _tilesize) (* (.y (.location _array_element)) _tilesize) 0.0)))))))

(event EventBeginPlay
  ;[1 1 1] Spawn actors
)

(event Collision|EventActorBeginOverlap
  (params (OtherActor :type Actor%20Object%20Reference)))

(event EventTick
  (params (DeltaSeconds :type Float%20%28single-precision%29)))

(fn ConstructionScript)